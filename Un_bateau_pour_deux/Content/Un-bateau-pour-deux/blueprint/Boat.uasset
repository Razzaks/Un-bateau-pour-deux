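; Physics-driven boat actor that moves and steers by applying forces to its mesh.
; On BeginPlay, four hover components are initialized with the boat mesh.
; Custom events apply forward force scaled by a speed input and yaw torque from an axis value, with a debug print while steering.
; The MoveForward and MoveRight axis events are empty, so nothing in this graph calls those custom events.
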(event `self.ReceiveBeginPlay`
  (bind _boatmesh (`self.BoatMesh`))
  ;[1 1 1] Récupère les hover
  (`/Game/Un-bateau-pour-deux/blueprint/HoverComponent.InitComponent` (`self.HoverComponent`) _boatmesh)
  (`/Game/Un-bateau-pour-deux/blueprint/HoverComponent.InitComponent` (`self.HoverComponent1`) _boatmesh)
  (`/Game/Un-bateau-pour-deux/blueprint/HoverComponent.InitComponent` (`self.HoverComponent2`) _boatmesh)
  (`/Game/Un-bateau-pour-deux/blueprint/HoverComponent.InitComponent` (`self.HoverComponent3`) _boatmesh))

(event `Throlle_Boat`
  ;[1 1 1] Throlle
  (`PrimitiveComponent.AddForce` (`self.BoatMesh`) (* (* (`SceneComponent.GetForwardVector` (`self.BoatMesh`)) 500000000.0) (`self.Input_Vistesse`)) "None" false))

(event `InputAxis|MoveForward`
  (params (AxisValue :type "Float (single-precision)"))
  ;[1 1 1] Throlle
)

(event `InputAxis|MoveRight`
  (params (AxisValue :type "Float (single-precision)"))
  ;[1 1 1] Steering
)

(event `Direction_Boat`
  (params (`Axis Value` :type "Float (double-precision)"))
  ;[1 1 1] Steering
  (`KismetSystemLibrary.PrintString` (`KismetStringLibrary.Conv_DoubleToString` (* (`KismetMathLibrary.SignOfFloat` (`self.GetInputAxisValue`)) (`self.Rotate`))))
  (`PrimitiveComponent.AddTorqueInDegrees` (`self.BoatMesh`) (`KismetMathLibrary.MakeVector` 0.0 0.0 (* `Axis Value` 180.0)) "None" true))

(fn `UserConstructionScript`)