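; Test helm (barre) actor that steers a boat from the mouse position.
; Each tick it compares cursor X to the viewport height cached at BeginPlay, rolls or spins the Cube by that ratio and passes it to Bateau's DirectionBoat.
; A click-and-hover rotation event using cursor deprojection, timeline rotations and a vehicle steering call remain, but their call sites or nodes are disconnected.
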(event `self.ReceiveBeginPlay`
  (bind _returnvalue (`GameplayStatics.GetPlayerController` 0))
  (set `self.max` (`KismetMathLibrary.Conv_IntToDouble` (`.SizeY` (`PlayerController.GetViewportSize` _returnvalue))))
  (bind _aswilliam_player_2 (cast `/Game/Un-bateau-pour-deux/blueprint/William_Player_2` (`Controller.K2_GetPawn` _returnvalue)))
  (set `self.Player` _aswilliam_player_2))

(event `self.ReceiveTick`
  (params (DeltaSeconds :type "Float (single-precision)"))
  ;[1 1 1] Roation de la barre en fonction position de la souris
  (bind _returnvalue (`WidgetLayoutLibrary.GetMousePositionOnViewport`))
  (bind _x (`KismetMathLibrary.BreakVector2D` _returnvalue))
  (`KismetSystemLibrary.PrintString` (`KismetStringLibrary.Conv_DoubleToString` _x))
  (bind _returnvalue_2 (/ (* DeltaSeconds (- (`self.max`) _x)) (`self.max`)))
  (`SceneComponent.K2_AddRelativeRotation` (`self.cube`) (* (struct :`Roll` 180.0) _returnvalue_2) false false)
  (`/Game/Un-bateau-pour-deux/blueprint/Boat.Direction_Boat` (`self.Bateau`) (* _returnvalue_2 90.0)))

(event `self.ReceiveActorBeginCursorOver`
  (set `self.Over` true))

(event `self.ReceiveActorEndCursorOver`)

(event `Rotation barre`
  ;[1 1 1] Rotation en fonction de la souris
  (if (and (`/Game/Un-bateau-pour-deux/blueprint/William_Player_2.LmbDown` (`self.Player`)) (`self.Over`))
    (`self.K2_SetActorRotation` (`KismetMathLibrary.MakeRotator` (* (.yaw (`KismetMathLibrary.Conv_VectorToRotator` (`.WorldDirection` (`PlayerController.DeprojectMousePositionToWorld` (`GameplayStatics.GetPlayerController` 0))))) 5.0)))))

(fn `UserConstructionScript`)